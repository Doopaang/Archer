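; BP_HPBar is an archer health bar Blueprint that displays an owner actor's HP through a widget component.
; Its UpdateBar event casts the widget to W_HPBar and sets the progress bar to the ratio of the owner's HP to MaxHP.
; The bar refreshes only when UpdateBar is called, and the construction script is empty.
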(event EventUpdateBar
  (bind _self self)
  (bind _owneractor (Variables|Default|GetOwnerActor _self))
  (bind _asw_hpbar (Utilities|Casting|CastToW_HPBar (UserInterface|GetWidget (Variables|Default|Getwidget))))
  (Progress|SetPercent (Variables|/Game/Archer/W_HPBar.W_HPBar_C|GetW_Progress _asw_hpbar) (/ (Math|Conversions|ToFloat(Integer) (Variables|/Script/Archer.UnitComponent|GetHP _owneractor)) (Math|Conversions|ToFloat(Integer) (Variables|/Script/Archer.UnitComponent|GetMaxHP _owneractor)))))

(fn ConstructionScript)